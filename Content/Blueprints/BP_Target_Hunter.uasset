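; BP_Target_Hunter is a scoring target actor that chases the player.
; Each Tick it moves toward player pawn 0 with a swept world offset, scaled by delta time and a random speed per axis, so its motion jitters.
; Interact spawns a green neon explosion, destroys the actor and returns its ScoreValue.
; BeginPlay stores the starting location in Origin, which these graphs never read.
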(event EventBeginPlay
  (Variables|Default|SetOrigin (Transformation|GetActorLocation)))

(event EventTick
  (params (DeltaSeconds :type Float%20%28single-precision%29))
  (bind _returnvalue (Math|Random|RandomFloatinRange 25.0 5e+01))
  (bind _returnvalue_2 (* DeltaSeconds _returnvalue))
  (Transformation|AddActorWorldOffset (* (* (Class|KismetMathLibrary|GetDirectionVector (Transformation|GetActorLocation) (Transformation|GetActorLocation (Game|Player|GetPlayerPawn 0))) (Math|Vector|MakeVector _returnvalue_2 _returnvalue_2 _returnvalue_2)) 5.0) true))

(fn ConstructionScript)

(fn Interact
  (Effects|SpawnEmitteratLocation "/Game/Effects/P_NeonExplosion_Green.P_NeonExplosion_Green" (Transformation|GetActorLocation))
  (Actor|DestroyActor)
  (return (Variables|Default|GetScoreValue)))