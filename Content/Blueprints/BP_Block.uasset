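; BP_Block is a randomized level block that dresses itself with a cover mesh, a colored point light and possible targets.
; NewFunction0 runs from both the Construction Script and BeginPlay, picking one of three light colors, then usually a cover mesh.
; Most rolls continue into SpawnTarget, which randomly spawns Wild plus PopUp, PopUp, ColorChange, Rotate, Hunter or nothing near the cover.
; The rotation and destroy-component nodes are unwired.
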(event EventBeginPlay
  (CallFunction|NewFunction0))

(fn ConstructionScript
  (bind _cover (Variables|Default|GetCover))
  (AddComponent|AddStaticMeshComponent (Components|GetOwner _cover) false (Math|Transform|MakeTransform "-260.000000,-190.000000, 0"))
  (Physics|SetSimulatePhysics _cover false)
  (CallFunction|NewFunction0))

(fn BuildBlock
  (params (Mesh :type Static%20Mesh%20Object%20Reference))
  (Components|StaticMesh|SetStaticMesh (Variables|Default|GetCover) Mesh)
  (switch int (Math|Random|RandomInteger 2)))

(fn SpawnTarget
  (bind _returnvalue (Math|Random|RandomUnitVector))
  (bind _cover (Variables|Default|GetCover))
  (bind _returnvalue_2 (Transformation|GetWorldLocation _cover))
  (bind _returnvalue_3 (Math|Vector|ClampVectorSize _returnvalue 0.2 0.9))
  (bind _returnvalue_4 (+ _returnvalue_2 "0,50.000000,100.000000"))
  (bind _returnvalue_5 (* _returnvalue_3 _returnvalue_2))
  (bind _returnvalue_6 (Math|Transform|MakeTransform _returnvalue_4))
  (bind _returnvalue_7 (+ _returnvalue_4 _returnvalue_5))
  (bind _returnvalue_8 (Math|Transform|TransformLocation _returnvalue_6 _returnvalue_2))
  (bind _returnvalue_9 (Math|Conversions|ToTransform(Vector) _returnvalue_8))
  (switch int (Math|Random|RandomInteger 7)
    (:Default
      _)
    (:0
      (Game|SpawnActorfromClass "/Game/Blueprints/BP_Target_Wild.BP_Target_Wild_C" (Math|Conversions|ToTransform(Vector) _returnvalue_7) "AdjustIfPossibleButAlwaysSpawn" 0 0)
      (Game|SpawnActorfromClass "/Game/Blueprints/BP_Target_PopUp.BP_Target_PopUp_C" (Math|Conversions|ToTransform(Vector) (+ _returnvalue_7 "0,0.000000,625.000000")) "AdjustIfPossibleButAlwaysSpawn" 0 0))
    (:1
      (Game|SpawnActorfromClass "/Game/Blueprints/BP_Target_PopUp.BP_Target_PopUp_C" _returnvalue_6 "AdjustIfPossibleButAlwaysSpawn" 0 0))
    (:2
      (Game|SpawnActorfromClass "/Game/Blueprints/BP_Target_ColorChange.BP_Target_ColorChange_C" _returnvalue_9 "AdjustIfPossibleButAlwaysSpawn" 0 0))
    (:3
      (Game|SpawnActorfromClass "/Game/Blueprints/BP_Target_Rotate.BP_Target_Rotate_C" (Math|Transform|MakeTransform (+ _returnvalue_4 "0,100.000000, 0")) "AdjustIfPossibleButAlwaysSpawn" 0 0))
    (:4
      (Game|SpawnActorfromClass "/Game/Blueprints/BP_Target_Hunter.BP_Target_Hunter_C" _returnvalue_9 "AdjustIfPossibleButAlwaysSpawn" 0 0)))
  (return))

(fn SpawnLight
  (switch int (Math|Random|RandomInteger 3)
    (:Default
      _)
    (:0
      (Rendering|Components|Light|SetLightColor (Variables|Default|GetPointLight) "(R=0.110688,G=0.555000,B=0.195516,A=1.000000)" true))
    (:1
      (Rendering|Components|Light|SetLightColor (Variables|Default|GetPointLight) "(R=0.870000,G=0.021750,B=0.294463,A=1.000000)" true))
    (:2
      (Rendering|Components|Light|SetLightColor (Variables|Default|GetPointLight) "(R=0.273318,G=0.219877,B=0.840000,A=1.000000)" true)))
  (return))

(fn NewFunction0
  (CallFunction|SpawnLight)
  (switch int (Math|Random|RandomInteger 23)
    (:Default
      (CallFunction|SpawnTarget :!label _label))
    (:0
      (CallFunction|BuildBlock "/Game/Meshes/Props/Cover/SM_Cover_High_Cnr_250.SM_Cover_High_Cnr_250")
      (goto _label))
    (:1
      (CallFunction|BuildBlock "/Game/Meshes/Props/Cover/SM_Cover_High_Cnr_250_002.SM_Cover_High_Cnr_250_002")
      (goto _label))
    (:2
      (CallFunction|BuildBlock "/Game/Meshes/Props/Cover/SM_Cover_High_Str_125.SM_Cover_High_Str_125")
      (goto _label))
    (:3
      (CallFunction|BuildBlock "/Game/Meshes/Props/Cover/SM_Cover_High_Str_250.SM_Cover_High_Str_250")
      (goto _label))
    (:4
      (CallFunction|BuildBlock "/Game/Meshes/Props/Cover/SM_Cover_High_Str_500.SM_Cover_High_Str_500")
      (goto _label))
    (:5
      (CallFunction|BuildBlock "/Game/Meshes/Props/Cover/SM_Cover_High_Str_125_002.SM_Cover_High_Str_125_002")
      (goto _label))
    (:6
      (CallFunction|BuildBlock "/Game/Meshes/Props/Cover/SM_Cover_High_Str_250_002.SM_Cover_High_Str_250_002")
      (goto _label))
    (:7
      (CallFunction|BuildBlock "/Game/Meshes/Props/Cover/SM_Cover_High_Str_500_002.SM_Cover_High_Str_500_002")
      (goto _label))
    (:8
      (CallFunction|BuildBlock "/Game/Meshes/Props/Cover/SM_Cover_Lw_Cnr_250.SM_Cover_Lw_Cnr_250")
      (goto _label))
    (:9
      (CallFunction|BuildBlock "/Game/Meshes/Props/Cover/SM_Cover_Lw_Str_125.SM_Cover_Lw_Str_125")
      (goto _label))
    (:10
      (CallFunction|BuildBlock "/Game/Meshes/Props/Cover/SM_Cover_Lw_Str_250.SM_Cover_Lw_Str_250")
      (goto _label))
    (:11
      (CallFunction|BuildBlock "/Game/Meshes/Props/Cover/SM_Cover_Lw_Str_500.SM_Cover_Lw_Str_500")
      (goto _label))
    (:12
      (CallFunction|BuildBlock "/Game/Meshes/Props/Cover/SM_Cover_Med_Cnr_250.SM_Cover_Med_Cnr_250")
      (goto _label))
    (:13
      (CallFunction|BuildBlock "/Game/Meshes/Props/Cover/SM_Cover_Med_Cnr_250_002.SM_Cover_Med_Cnr_250_002")
      (goto _label))
    (:14
      (CallFunction|BuildBlock "/Game/Meshes/Props/Cover/SM_Cover_Med_Str_125.SM_Cover_Med_Str_125")
      (goto _label))
    (:15
      (CallFunction|BuildBlock "/Game/Meshes/Props/Cover/SM_Cover_Med_Str_500_002.SM_Cover_Med_Str_500_002")
      (goto _label))
    (:16
      (CallFunction|BuildBlock "/Game/Meshes/Props/Cover/SM_Cover_Med_Str_125_002.SM_Cover_Med_Str_125_002")
      (goto _label))
    (:17
      _))
  (return))