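; A pop-up shooting target that rises from its placed spot and awards a score when hit through Interact.
; After a random delay of a few seconds from BeginPlay, the UpAndDown timeline offsets it vertically from its stored origin.
; Interact spawns a green neon explosion, destroys the actor and returns its ScoreValue.
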(event EventBeginPlay
  (Variables|Default|SetOrigin (Transformation|GetActorLocation))
  (Utilities|FlowControl|Delay (Math|Random|RandomFloatinRange 2.0 6.0))
  (bind _data (Timeline|UpAndDown PlayFromStart)
    (:Update
      (Transformation|SetActorLocation (+ (* "0, 0,200.000000" _data) (Variables|Default|GetOrigin)) false false))))

(fn ConstructionScript)

(fn Interact
  (Effects|SpawnEmitteratLocation "/Game/Effects/P_NeonExplosion_Green.P_NeonExplosion_Green" (Transformation|GetActorLocation))
  (Actor|DestroyActor)
  (return (Variables|Default|GetScoreValue)))