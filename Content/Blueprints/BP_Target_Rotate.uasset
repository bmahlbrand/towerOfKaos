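; BP_Target_Rotate is a moving target that, on Interact, spawns a green neon explosion, destroys itself and returns a score value.
; On BeginPlay a timeline positions it along a fixed sideways-and-up offset from its starting location.
; Tick also calls Orbit, adding a swept, rotated offset to its location, but a zero multiplier keeps the angle from advancing.
; The random-delay timeline replay is never executed.
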(event EventBeginPlay
  (Variables|Default|SetOrigin (Transformation|GetActorLocation))
  (bind _data (Timeline|Timeline_0 Play)
    (:Update
      (Transformation|SetActorLocation (+ (* "0,75.000000,100.000000" _data) (Variables|Default|GetOrigin)) false false))))

(event EventTick
  (params (DeltaSeconds :type Float%20%28single-precision%29))
  (CallFunction|Orbit DeltaSeconds))

(fn ConstructionScript)

(fn Orbit
  (params (A :type Float%20%28single-precision%29))
  (bind _output_get (Variables|Default|SetCurrentRotation (+ (* 0.0 (Variables|Default|GetRotationSpeed)) (Variables|Default|GetCurrentRotation))))
  (Transformation|SetActorRelativeLocation (+ (Transformation|GetActorLocation) (Math|Vector|RotateVectorAroundAxis "10.000000, 0, 0" _output_get "0.000000,1.000000,0.000000")) true)
  (return))

(fn Interact
  (Effects|SpawnEmitteratLocation "/Game/Effects/P_NeonExplosion_Green.P_NeonExplosion_Green" (Transformation|GetActorLocation))
  (Actor|DestroyActor)
  (return (Variables|Default|GetScoreValue)))