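; A shootable-style target actor that periodically changes color and awards points based on its current color when interacted with.
; From BeginPlay, ChangeType randomly picks gold, green or yellow, setting the mesh material and matching ScoreValue (yellow is a penalty), then re-calls itself after a random delay.
; Interact spawns a green neon explosion regardless of color, destroys the actor and returns the current score to the caller.
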(event Custom|ChangeType
  (switch int (Math|Random|RandomIntegerinRange 0 2)
    (:0
      (Rendering|Material|SetMaterial (Variables|Default|GetTarget) 0 "/Game/Materials/Targets/MI_Targets_Gold.MI_Targets_Gold")
      (Variables|Default|SetScoreValue 10))
    (:1
      (Rendering|Material|SetMaterial (Variables|Default|GetTarget) 0 "/Game/Materials/Targets/MI_Targets_Green.MI_Targets_Green")
      (Variables|Default|SetScoreValue 5))
    (:2
      (Rendering|Material|SetMaterial (Variables|Default|GetTarget) 0 "/Game/Materials/Targets/MI_Targets_Yellow.MI_Targets_Yellow")
      (Variables|Default|SetScoreValue -5)))
  (Utilities|FlowControl|Delay (Math|Random|RandomFloatinRange 2.0 6.0))
  (CallFunction|ChangeType))

(event EventBeginPlay
  (CallFunction|ChangeType))

(fn ConstructionScript)

(fn Interact
  (Effects|SpawnEmitteratLocation "/Game/Effects/P_NeonExplosion_Green.P_NeonExplosion_Green" (Transformation|GetActorLocation))
  (Actor|DestroyActor)
  (return (Variables|Default|GetScoreValue)))