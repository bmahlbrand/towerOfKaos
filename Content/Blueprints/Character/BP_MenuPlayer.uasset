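; BP_MenuPlayer is the VR menu player, which selects BP_PlayButton actors by gaze and can fade to black.
; Each Tick moves the spring arm to the camera and line-traces forward, building frame-based hover progress while the same button stays hit.
; Progress drives the billboard reticle material, and full progress calls Select once.
; FadeToBlack runs a timeline driving opacity on the BlindingBox's dynamic material.
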(event Custom|FadeToBlack
  ;[1 1 1] Layout Utility: Fade to Black
  (bind _data (Timeline|FadeToFullOpacity Play)
    (:Update
      (Rendering|Material|SetScalarParameterValue (Variables|Default|GetFadeDMI) "FadeOpacity" _data :!class /Script/Engine.MaterialInstanceDynamic))))

(event EventTick
  (params (DeltaSeconds :type Float%20%28single-precision%29))
  (bind (_location _forward_vector) (CallFunction|GetPlayerVRCameraProperties))
  (Transformation|SetWorldLocation (Variables|Default|GetSpringArm) _location false false)
  (bind _outhit (Collision|LineTraceByChannel _location (+ _location (* _forward_vector 5e+03)) "TraceTypeQuery1" false 0 "None"))
  (Utilities|FlowControl|Sequence
    (:then_0
      (if (== (Variables|Default|GetLastTraceActor) (.HitActor (Collision|BreakHitResult _outhit)))
        (bind _asbp_play_button (Utilities|Casting|CastToBP_PlayButton (.HitActor (Collision|BreakHitResult _outhit))))
        (bind _output_get (Variables|Default|SetHoverProgress (+ (Variables|Default|GetHoverProgress) 0.01)))
        (if (>= _output_get 1.0)
          (Utilities|FlowControl|DoOnce false
            (:Completed
              (Default|Select _asbp_play_button))))
        (else
          (Variables|Default|SetHoverProgress 0.0))))
    (:then_1
      (Variables|Default|SetLastTraceActor (.HitActor (Collision|BreakHitResult _outhit)))
      (Rendering|Material|SetScalarParameterValue (Variables|Default|GetReticleDMI) "Progress" (Variables|Default|GetHoverProgress) :!class /Script/Engine.MaterialInstanceDynamic))))

(fn ConstructionScript
  (CallFunction|CreateFadeDMI)
  (bind _dynamic_material (CallFunction|CreateDynamicBillboardMaterial (Variables|Default|GetMaterialBillboard)))
  (Variables|Default|SetReticleDMI _dynamic_material))

(fn CreateFadeDMI
  (bind _returnvalue (Rendering|Material|CreateDynamicMaterialInstance (Variables|Default|GetBlindingBox) 0 "/Game/Materials/UI/M_Menu_Fade.M_Menu_Fade" :!class /Script/Engine.PrimitiveComponent))
  (Variables|Default|SetFadeDMI _returnvalue))