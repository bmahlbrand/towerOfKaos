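; BP_Grid generates a multi-floor block building at BeginPlay, stacking one grid per floor at a fixed height step.
; Each cell spawns a BP_Block, except a fixed stairwell cell that gets stairs, plus an empty floor on the first level.
; BP_Wall actors line all four edges, rotated on two sides; one side adds the floor offset twice.
; Random size ranges have equal min and max, and BuildWall is an empty stub.
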(event EventBeginPlay
  (for _index (range 0 (Variables|Default|GetFloors))
    (bind _output_get (Variables|Default|SetCurrentFloorOffset (* "0, 0,650.000000" _index)))
    (Variables|Default|SetWidth (Math|Random|RandomIntegerinRange 7 7))
    (Variables|Default|SetHeight (Math|Random|RandomIntegerinRange 5 5))
    (for _index_2 (range 0 (Variables|Default|GetWidth))
      (for _index_3 (range 0 (Variables|Default|GetHeight))
        (if (== _index_2 1)
          (if (== _index_3 1)
            (Game|SpawnActorfromClass "/Game/Blueprints/BP_Block_Stairs.BP_Block_Stairs_C" (Math|Conversions|ToTransform(Vector) (+ (* "500.000000, 0,0.000000" _index_2) (* "0,500.000000,0.000000" _index_3) _output_get)) "AdjustIfPossibleButAlwaysSpawn" 0 0)
            (if (== _index 0)
              (Game|SpawnActorfromClass "/Game/Blueprints/BP_Block_EmptyFloor.BP_Block_EmptyFloor_C" (Math|Conversions|ToTransform(Vector) (+ (* "500.000000, 0,0.000000" _index_2) (* "0,500.000000,0.000000" _index_3) _output_get)) "Undefined" 0 0))
            (else
              (Game|SpawnActorfromClass "/Game/Blueprints/BP_Block.BP_Block_C" (Math|Conversions|ToTransform(Vector) (+ (* "500.000000, 0,0.000000" _index_2) (* "0,500.000000,0.000000" _index_3) _output_get)) "Undefined" 0 0 :!label _label)))
          (else
            (goto _label)))))
    (CallFunction|BuildWall)
    (for _index_4 (range 0 (Variables|Default|GetWidth))
      (Utilities|FlowControl|Sequence
        (:then_0
          (bind _returnvalue (Game|SpawnActorfromClass "/Game/Blueprints/BP_Wall.BP_Wall_C" (Math|Conversions|ToTransform(Vector) (+ (* "500.000000,0.000000, 0" _index_4) (+ (* "0.000000,500.000000, 0" (Variables|Default|GetHeight)) (* "-500.000000,-500.000000, 0" 1) _output_get) _output_get)) "Undefined" 0 0))
          (Transformation|SetRelativeRotation (Variables|/Game/Blueprints/BP_Wall.BP_Wall_C|GetDefaultSceneRoot _returnvalue) "0.000000,90.000000, 0" false false))
        (:then_1
          (bind _returnvalue_2 (Game|SpawnActorfromClass "/Game/Blueprints/BP_Wall.BP_Wall_C" (Math|Conversions|ToTransform(Vector) (+ (* "500.000000,0.000000, 0" _index_4) (* "-500.000000,-500.000000, 0" 1) _output_get)) "Undefined" 0 0))
          (Transformation|SetRelativeRotation (Variables|/Game/Blueprints/BP_Wall.BP_Wall_C|GetDefaultSceneRoot _returnvalue_2) "0,90.000000, 0" false false))))
    (for _index_5 (range 0 (Variables|Default|GetHeight))
      (Utilities|FlowControl|Sequence
        (:then_0
          (Game|SpawnActorfromClass "/Game/Blueprints/BP_Wall.BP_Wall_C" (Math|Conversions|ToTransform(Vector) (+ (* "0.000000,500.000000, 0" _index_5) (* "500.000000, 0, 0" (Variables|Default|GetWidth)) _output_get)) "Undefined" 0 0))
        (:then_1
          (Game|SpawnActorfromClass "/Game/Blueprints/BP_Wall.BP_Wall_C" (Math|Conversions|ToTransform(Vector) (+ (* "0.000000,500.000000, 0" _index_5) (* "-500.000000, 0, 0" 1) _output_get)) "Undefined" 0 0))))))

(fn ConstructionScript)

(fn BuildWall)